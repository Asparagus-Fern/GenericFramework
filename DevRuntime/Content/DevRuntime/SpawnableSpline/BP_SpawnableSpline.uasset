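; BP_SpawnableSpline is a spline-driven spawning Blueprint that attaches spawn handles to its splines.
; After the parent construction script runs, it calls UpdateSpawnSpline, which triggers AddSpawnableSplineContainer.
; That event creates one AC_SpawnableSplineHandle per spline component, passes it the shared SpawnableSplineContainer and ContainerGenerationOptions, and appends it to SpawnableSplineHandles.
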(event Custom|UpdateSpawnSpline
  (CallFunction|AddSpawnableSplineContainer))

(event Custom|AddSpawnableSplineContainer
  (for _array_element (Variables|Default|GetSplineComponents)
    (bind _returnvalue (Game|AddComponentbyClass "/DevRuntime/DevRuntime/SpawnableSpline/AC_SpawnableSplineHandle.AC_SpawnableSplineHandle_C" _array_element (Variables|Default|GetSpawnableSplineContainer) (Variables|Default|GetContainerGenerationOptions)))
    (Utilities|Array|Add (Variables|Default|GetSpawnableSplineHandles) _returnvalue)))

(event EventTick
  (params (DeltaSeconds :type Float%20%28single-precision%29)))

(fn ConstructionScript
  (|CallParentFunction)
  (CallFunction|UpdateSpawnSpline))