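; BP_MovablePoint is a point actor with a Camera component whose field of view is set from the FieldOfView variable.
; The construction script applies that value, then passes the actor's rotation through RotatorSafe and sets it back, which BeginPlay repeats at runtime.
; A Refresh boolean resets itself during construction, acting as an editor toggle to rerun the script.
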(event EventBeginPlay
  (Transformation|SetActorRotation (Class|BPFunctionsMath|RotatorSafe (Transformation|GetActorRotation))))

(fn ConstructionScript
  (if (Variables|Default|GetRefresh)
    (Variables|Default|SetRefresh false))
  (Utilities|FlowControl|Sequence
    (:then_0
      (Camera|SetFieldOfView (Variables|Default|GetCamera) (Variables|Default|GetFieldOfView)))
    (:then_1
      (Transformation|SetActorRotation (Class|BPFunctionsMath|RotatorSafe (Transformation|GetActorRotation))))))