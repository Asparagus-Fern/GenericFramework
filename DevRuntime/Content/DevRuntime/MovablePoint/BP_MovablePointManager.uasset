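; Manager that animates transitions between BP_MovablePoint actors, requested by index or name, and broadcasts the result through OnMoving.
; The construction script collects and indexes all points, optionally drawing debug splines between every pair.
; Each move adds a three-point spline bent by SplineBase angle and height, which a timeline samples for location while lerping rotation.
; A move requested mid-transition starts from the current interpolated location and rotation.
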(event Custom|MoveToPointByIndex
  (params (Index :type Integer))
  (bind _points (Variables|Default|GetPoints))
  (bind _output (Utilities|Array|Get(acopy) _points Index))
  (if (CallFunction|CanMove Index)
    (if (Variables|Default|GetIsMoving)
      (Variables|Default|SetOriginMovingResult (Variables|Default|GetCurrentMovingResult))
      (else
        (Variables|Default|SetIsMoving true)
        (Variables|Default|SetOriginMovingResult (Utilities|Struct|MakeS_MovingResult 0.0 (Transformation|GetActorLocation (Utilities|Array|Get(acopy) _points (Variables|Default|GetCurrentPointIndex))) (Transformation|GetActorRotation (Utilities|Array|Get(acopy) _points (Variables|Default|GetCurrentPointIndex))) (Utilities|Array|Get(acopy) _points (Variables|Default|GetCurrentPointIndex))))))
    (bind _splinecomponent (CallFunction|CreateSplineComponent (Utilities|Struct|MakeS_SplineLocation (Variables|Default|GetSplineBase) (Utilities|Struct|BreakS_MovingResult (Variables|Default|GetOriginMovingResult)) (Transformation|GetActorLocation _output))))
    (bind _alpha (Timeline|Timeline PlayFromStart)
      (:Update
        (bind _output_get (Variables|Default|SetCurrentMovingResult (Utilities|Struct|MakeS_MovingResult _alpha (Spline|GetLocationatTime _splinecomponent _alpha "World" false) (Math|Rotator|Lerp(Rotator) (.Rotation (Utilities|Struct|BreakS_MovingResult (Variables|Default|GetOriginMovingResult))) (Transformation|GetActorRotation _output) _alpha) _output)))
        (Default|CallOnMoving _output_get))
      (:Finished
        (Variables|Default|SetIsMoving false)
        (Variables|Default|SetCurrentPointIndex Index)
        (Variables|Default|SetOriginMovingResult "")))))

(event Custom|MoveToPointByName
  (params (Name :type Name))
  (for (_array_element _array_index) (Variables|Default|GetPoints)
    (if (== (Variables|/DevRuntime/DevRuntime/MovablePoint/BP_MovablePoint.BP_MovablePoint_C|GetName _array_element) Name)
      (CallFunction|MovetoPointbyIndex _array_index))))

(fn ConstructionScript
  (if (Variables|Default|GetRefresh)
    (Variables|Default|SetRefresh false))
  (Utilities|FlowControl|Sequence
    (:then_0
      (bind _outactors (Actor|GetAllActorsOfClass "/DevRuntime/DevRuntime/MovablePoint/BP_MovablePoint.BP_MovablePoint_C"))
      (bind _output_get (Variables|Default|SetPoints _outactors))
      (for (_array_element _array_index) _output_get
        (Variables|/DevRuntime/DevRuntime/MovablePoint/BP_MovablePoint.BP_MovablePoint_C|SetIndex _array_element _array_index)))
    (:then_1
      (if (Variables|Default|GetDebugSpline)
        (for (_array_element_2 _array_index_2) (Variables|Default|GetPoints)
          (for (_array_element_3 _array_index_3) (Variables|Default|GetPoints)
            (if (!= _array_index_3 _array_index_2)
              (CallFunction|CreateSplineComponent (Utilities|Struct|MakeS_SplineLocation (Variables|Default|GetSplineBase) (Transformation|GetActorLocation _array_element_2) (Transformation|GetActorLocation _array_element_3))))))))))

(fn CanMove
  (params (Index :type Integer))
  (return (and (< Index (Utilities|Array|Length (Variables|Default|GetPoints))) (!= (Variables|Default|GetCurrentPointIndex) Index))))

(fn CreateSplineComponent
  (params (SplineLocation :type S%20Spline%20Location%20Structure))
  (bind (_splinebase _startlocation _endlocation) (Utilities|Struct|BreakS_SplineLocation SplineLocation))
  (bind _returnvalue (Game|AddComponentbyClass "/Script/Engine.SplineComponent" false))
  (Spline|ClearSplinePoints _returnvalue false)
  (Spline|AddSplinePoint _returnvalue _startlocation "World" false)
  (Spline|AddSplinePoint _returnvalue (CallFunction|GetMiddleLocation _splinebase _startlocation _endlocation) "World" false)
  (Spline|AddSplinePoint _returnvalue _endlocation "World" true)
  (return _returnvalue))

(fn GetMiddleLocation
  (params (SplineBase :type S%20Spline%20Base%20Structure) (LocationA :type Vector) (LocationB :type Vector))
  (bind (_height _angle) (Utilities|Struct|BreakS_SplineBase SplineBase))
  (return (+ (* (Math|Vector|RotateVector (Math|Vector|Normalize (- LocationB LocationA)) (Math|Rotator|MakeRotator 0.0 0.0 _angle)) (/ (* (Math|Vector|Distance(Vector) LocationA LocationB) 0.5) (Math|Trig|Cos(Degrees) _angle))) LocationA (Math|Vector|MakeVector 0.0 0.0 _height))))