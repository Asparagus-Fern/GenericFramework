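; Actor that builds a spline through named, indexed points and animates a location along it between them.
; Construction inserts a computed middle point before each configured point and re-indexes the list.
; MoveToPoint, also reachable by name or test keys, maps a Duration-scaled timeline onto spline time, restarting from the current location if interrupted.
; It fires start and finish dispatchers, but the per-update OnMoving broadcast and test pawn binding are disconnected.
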(event Custom|MoveToPoint
  (params (Index :type Integer))
  (bind _connectionsplinepoint (CallFunction|GetConnectionSplinePointbyIndex Index))
  ;[0.4766 0 1] 移动到某个点
  (if (CallFunction|CanMove Index)
    (if (Variables|ConnectionSpline|GetIsMoving)
      (Variables|ConnectionSpline|SetOriginLocation (Variables|ConnectionSpline|GetCurrentLocation))
      (else
        (Variables|ConnectionSpline|SetIsMoving true)
        (Default|CallOnMovingStart)
        (Variables|ConnectionSpline|SetOriginLocation (Utilities|Struct|BreakS_SplineMovingPoint (Variables|ConnectionSpline|GetCurrentConnectionSplinePoint)))))
    (Variables|ConnectionSpline|SetCurrentConnectionSplinePoint _connectionsplinepoint)
    (bind _alpha (Timeline|Timeline PlayFromStart)
      (:Update
        (Variables|ConnectionSpline|SetCurrentLocation (Spline|GetLocationatTime (Utilities|Array|Get(acopy) (Variables|Default|GetSplineComponents)) (Math|Float|MapRangeClamped _alpha 0.0 1.0 (.Time (CallFunction|GetSplineTimebyLocation (Variables|ConnectionSpline|GetOriginLocation))) (.Time (CallFunction|GetSplineTimebyIndex (.Index (Utilities|Struct|BreakS_SplineMovingPoint _connectionsplinepoint))))) "Local" false)))
      (:Finished
        (Default|CallOnMovingFinish)
        (Variables|ConnectionSpline|SetIsMoving false)))))

(event Custom|OnMoving_Event
  (params (Result :type Boolean) (MovingResult :type S%20Moving%20Result%20Structure))
  ;[1 0 0.1875] 测试
  (if Result
    (Transformation|SetActorLocation (Game|Player|GetPlayerPawn 0) (.Location (Utilities|Struct|BreakS_MovingResult MovingResult)) false false)))

(event EventBeginPlay
  (Components|Timeline|SetPlayRate (Variables|Default|GetTimeline) (/ 1.0 (Variables|ConnectionSpline|GetDuration))))

(event Input|KeyboardEvents|1
  (params (Key :type Key%20Structure :default "None"))
  ;[0.2891 1 0] 测试
  (:Pressed
    (CallFunction|MovetoPoint 1)))

(event Input|KeyboardEvents|2
  (params (Key :type Key%20Structure :default "None"))
  ;[0.2891 1 0] 测试
  (:Pressed
    (CallFunction|MovetoPoint 2)))

(event Input|KeyboardEvents|0
  (params (Key :type Key%20Structure :default "None"))
  ;[0.2891 1 0] 测试
  (:Pressed
    (CallFunction|MovetoPoint)))

(fn ConstructionScript
  (Utilities|Array|Clear (Variables|Default|GetSplineLocations))
  (CallFunction|AddSplineComponent))

(fn AddSplineComponent
  (params (SplineLocation :type S%20Spline%20Location%20Structure))
  (bind _connectionspline (Variables|ConnectionSpline|GetConnectionSpline))
  (bind (_splinebase _camerasplinepoints) (Utilities|Struct|BreakS_SplineMoving _connectionspline))
  (bind _returnvalue (Game|AddComponentbyClass "/Script/Engine.SplineComponent" false))
  (bind _output_get (LocalVariables|SetCameraSplineComponent _returnvalue))
  (Utilities|Array|Add (Variables|Default|GetSplineComponents) _output_get)
  (Spline|ClearSplinePoints _output_get false)
  (Spline|AddSplinePoint _output_get (Math|Vector|VectorZero) "Local" false)
  (for (_array_element _array_index) _camerasplinepoints
    (Utilities|Array|Add (LocalVariables|GetLocalPoints) (Utilities|Struct|MakeS_SplineMovingPoint _array_index (.PointName (Utilities|Struct|BreakS_SplineMovingPoint _array_element)) (.Location (Utilities|Struct|BreakS_SplineMovingPoint _array_element))))
    (Spline|AddSplinePoint (LocalVariables|GetCameraSplineComponent) (CallFunction|GetMiddleLocation _splinebase (LocalVariables|GetLocationA) (.Location (Utilities|Struct|BreakS_SplineMovingPoint _array_element))) "Local" false)
    (Spline|AddSplinePoint (LocalVariables|GetCameraSplineComponent) (.Location (Utilities|Struct|BreakS_SplineMovingPoint _array_element)) "Local" true)
    (LocalVariables|SetLocationA (.Location (Utilities|Struct|BreakS_SplineMovingPoint _array_element))))
  (Utilities|Struct|SetmembersinS_SplineMoving _connectionspline (LocalVariables|GetLocalPoints)))

(fn CanMove
  (params (Index :type Integer))
  (return (!= Index (Utilities|Struct|BreakS_SplineMovingPoint (Variables|ConnectionSpline|GetCurrentConnectionSplinePoint)))))

(fn GetConnectionSplinePointbyIndex
  (params (Index :type Integer))
  (for _array_element (.CameraSplinePoints (Utilities|Struct|BreakS_SplineMoving (Variables|ConnectionSpline|GetConnectionSpline)))
    (if (== (.Index (Utilities|Struct|BreakS_SplineMovingPoint _array_element)) Index)
      (return _array_element))))

(fn GetConnectionSplinePointbyName
  (params (PointName :type Name))
  (for _array_element (.CameraSplinePoints (Utilities|Struct|BreakS_SplineMoving (Variables|ConnectionSpline|GetConnectionSpline)))
    (if (== (.PointName (Utilities|Struct|BreakS_SplineMovingPoint _array_element)) PointName)
      (return _array_element))))

(fn GetSplineLocationbyIndex
  (params (Index :type Integer))
  (bind _splinecomponents (Variables|Default|GetSplineComponents))
  (bind _output (Utilities|Array|Get(acopy) _splinecomponents))
  (Utilities|IsValid _output
    (:Is%20Valid
      (return true (Spline|GetLocationatSplinePoint _output (* Index 2) "Local")))
    (:Is%20Not%20Valid
      (return false "0, 0, 0"))))

(fn GetSplineTimebyIndex
  (params (Index :type Integer))
  (bind _splinecomponents (Variables|Default|GetSplineComponents))
  (bind _output (Utilities|Array|Get(acopy) _splinecomponents))
  (Utilities|IsValid _output
    (:Is%20Valid
      (return true (Class|SplineComponent|GetTimeatDistanceAlongSpline _output (Spline|GetDistanceAlongSplineatSplinePoint _output (* (+ Index 1) 2)))))
    (:Is%20Not%20Valid
      (return false 0.0))))

(fn GetSplineTimebyLocation
  (params (Location :type Vector))
  (bind _splinecomponents (Variables|Default|GetSplineComponents))
  (bind _output (Utilities|Array|Get(acopy) _splinecomponents))
  (Utilities|IsValid _output
    (:Is%20Valid
      (return true (Class|SplineComponent|GetTimeatDistanceAlongSpline _output (Class|SplineComponent|GetDistanceAlongSplineatLocation _output Location "Local"))))
    (:Is%20Not%20Valid
      (return false 0.0))))

(fn MovetoPointbyName
  (params (Name :type Name))
  (for _array_element (Utilities|Struct|BreakS_SplineMoving (Variables|ConnectionSpline|GetConnectionSpline))
    (if (and (== (.PointName (Utilities|Struct|BreakS_SplineMovingPoint _array_element)) Name) (!= (.PointName (Utilities|Struct|BreakS_SplineMovingPoint _array_element)) ""))
      (CallFunction|MovetoPoint (.Index (Utilities|Struct|BreakS_SplineMovingPoint _array_element))))))