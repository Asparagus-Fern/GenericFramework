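; BP_TestActionNode is a test action node that exercises the ActiveNode subsystem's registration and switching flow.
; On BeginPlay it binds to the subsystem's node-register delegate and makes ActiveNode.Test the active node, without reinitialization, when that tag registers.
; Its login, init, logout and register events only print debug messages, with registration also showing the node's gameplay tag.
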(event Custom|OnActionNodeRegister_Event
  (params (NodeTag :type Gameplay%20Tag%20Structure%20%28by%20ref%29))
  (if (== NodeTag "(TagName=\"ActiveNode.Test\")")
    (Class|ActiveNodeSubsystem|ChangeActiveNodeto (Subsystems|GetActiveNodeSubsystem) "(TagName=\"ActiveNode.Test\")" false)))

(event EventBeginPlay
  (EventDispatchers|AssignOnActionNodeRegister (Subsystems|GetActiveNodeSubsystem) (delegate Custom|OnActionNodeRegister_Event)))

(event EventTick
  (params (DeltaSeconds :type Float%20%28single-precision%29)))

(event EventLoginNode
  (Development|PrintString "node login"))

(event EventInitNode
  (Development|PrintString "node Init"))

(event EventLogoutNode
  (Development|PrintString "node Logout"))

(event EventRegisterNode
  (Development|PrintString (Utilities|String|Append "rgister node -> " (GameplayTags|GetDebugStringfromGameplayTag (Variables|Default|GetNodeTag)))))

(fn ConstructionScript)