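; BP_Cylinder is a 3D bar-chart cylinder that visualizes a value within a min/max range, with a floating text label.
; Update sets the mesh, scales its height by the normalized value, and places Text3D just above the top, showing either value with unit or percentage.
; The construction script calls Update, and BeginPlay runs a GrowUp timeline that animates the value from minimum to target, refreshing each tick.
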(event Custom|Update
  (bind _text3d (Variables|Default|GetText3D))
  (bind _scalexy (Variables|Default|GetScaleXY))
  (Utilities|FlowControl|Sequence
    (:then_0
      (Components|StaticMesh|SetStaticMesh (Variables|Default|GetStaticMesh) (Variables|Default|GetMesh)))
    (:then_1
      (Transformation|SetRelativeScale3D (Variables|Default|GetStaticMesh) (Math|Vector|MakeVector _scalexy _scalexy (CallFunction|GetCylinderHeightScaleZ))))
    (:then_2
      (Transformation|SetRelativeLocation _text3d (Math|Vector|MakeVector 0.0 0.0 (+ (CallFunction|GetCylinderHeight) 1e+01)) false false)
      (Variables|/Script/Text3D.Text3DComponent|SetText _text3d (CallFunction|GetCylinderText)))))

(event Custom|PlayGrowUp
  (Variables|Default|SetGrowUpValue (Variables|Default|GetValue))
  (Variables|Default|SetValue 0.0)
  (bind _alpha (Timeline|GrowUp PlayFromStart)
    (:Update
      (Variables|Default|SetValue (Math|Float|Lerp (Variables|Default|GetMinValue) (Variables|Default|GetGrowUpValue) _alpha))
      (CallFunction|Update))))

(event EventBeginPlay
  (CallFunction|PlayGrowUp))

(fn ConstructionScript
  (CallFunction|Update))

(fn GetValueNormalize
  (return (Math|Float|MapRangeClamped (Variables|Default|GetValue) (Variables|Default|GetMinValue) (Variables|Default|GetMaxValue) 0.0 1.0)))

(fn GetCylinderText
  (switch Utilities|FlowControl|Switch|SwitchonE_TextFormat (Variables|Default|GetTextFormat)
    (:NewEnumerator0
      (return (Utilities|Text|FormatText "{Value}{Unit}" (Utilities|Text|ToText(Float) (Math|Float|Clamp(Float) (Variables|Default|GetValue) (Variables|Default|GetMinValue) (Variables|Default|GetMaxValue)) "HalfToEven" false false 1 324 (Variables|Default|GetMinimumFractionalDigits) (Variables|Default|GetMaximumFractionalDigits)) (Variables|Default|GetUnitText))))
    (:NewEnumerator1
      (return (Utilities|Text|FormatText "{Value}%" (Utilities|Text|ToText(Float) (* (CallFunction|GetValueNormalize) 1e+02) "HalfToEven" false false 1 324 (Variables|Default|GetMinimumFractionalDigits) (Variables|Default|GetMaximumFractionalDigits)))))))

(fn GetCylinderHeight
  (return (* (* (CallFunction|GetValueNormalize) 1e+02) (/ (Variables|Default|GetMaxValueHeight) 1e+02))))

(fn GetCylinderHeightScaleZ
  (return (* (CallFunction|GetValueNormalize) (/ (Variables|Default|GetMaxValueHeight) 1e+02))))