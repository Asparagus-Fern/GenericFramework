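; BP_Grid is an actor that draws a two-axis grid or chart frame with a scaled background and unit labels.
; The construction script calls Update, which stretches both axis meshes from the origin along actor forward and negated right by GridSize.
; It also places and rotates the unit labels beyond each axis end and scales the background.
; Axis values can be appended, but UpdateAxisValue is empty and the tick-spacing logic is unfinished and disconnected.
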(event Custom|Update
  (CallFunction|DrawAxis)
  (CallFunction|DrawUnit)
  (CallFunction|DrawBackground)
  (CallFunction|SetAxisXUnitText (Variables|Default|GetAxisXUnitText))
  (CallFunction|SetAxisYUnitText (Variables|Default|GetAxisYUnitText)))

(event Custom|DrawAxis
  (for _index (range 0 1)
    (SplineMesh|SetStartPosition (Utilities|Select :Index _index :Option%200 (Variables|Default|GetAxisX) :Option%201 (Variables|Default|GetAxisY)) (CallFunction|GetOriginLocation) false)
    (SplineMesh|SetEndPosition (Utilities|Select :Index _index :Option%200 (Variables|Default|GetAxisX) :Option%201 (Variables|Default|GetAxisY)) (Utilities|Select :Index _index :Option%200 (CallFunction|GetAxisXEndLocation) :Option%201 (CallFunction|GetAxisYEndLocation)) true)))

(event Custom|UpdateAxisValue)

(event Custom|DrawUnit
  (bind _result (CallFunction|GetAxisXEndLocation))
  (bind _result_2 (CallFunction|GetAxisYEndLocation))
  (bind _result_3 (CallFunction|GetOriginLocation))
  (bind _returnvalue (Math|Rotator|FindLookatRotation _result_3 _result))
  (for _index (range 0 1)
    (Transformation|SetRelativeRotation (Utilities|Select :Index _index :Option%200 (Variables|Default|GetAxisXUnit) :Option%201 (Variables|Default|GetAxisYUnit)) (Math|Rotator|MakeRotator (.roll (Utilities|Select :Index _index :Option%200 (Math|Rotator|MakeRotator (.roll _returnvalue) (.pitch _returnvalue) (+ (.yaw _returnvalue) -9e+01)) :Option%201 (Math|Rotator|FindLookatRotation _result_3 _result_2))) (+ (.pitch (Utilities|Select :Index _index :Option%200 (Math|Rotator|MakeRotator (.roll _returnvalue) (.pitch _returnvalue) (+ (.yaw _returnvalue) -9e+01)) :Option%201 (Math|Rotator|FindLookatRotation _result_3 _result_2))) -9e+01) (.yaw (Utilities|Select :Index _index :Option%200 (Math|Rotator|MakeRotator (.roll _returnvalue) (.pitch _returnvalue) (+ (.yaw _returnvalue) -9e+01)) :Option%201 (Math|Rotator|FindLookatRotation _result_3 _result_2)))) false false)
    (Transformation|SetRelativeLocation (Utilities|Select :Index _index :Option%200 (Variables|Default|GetAxisXUnit) :Option%201 (Variables|Default|GetAxisYUnit)) (+ (Utilities|Select :Index _index :Option%200 _result :Option%201 _result_2) (* (Utilities|Select :Index _index :Option%200 (CallFunction|GetAxisXDirection) :Option%201 (CallFunction|GetAxisYDirection)) 3e+01)) false false)))

(event Custom|DrawBackground
  (bind _gridsize (Variables|Default|GetGridSize))
  (bind _returnvalue (/ _gridsize 1e+02))
  (Transformation|SetRelativeScale3D (Variables|Default|GetBackground) (Math|Vector|MakeVector (.x _returnvalue) (.y _returnvalue) 1.0)))

(event Custom|SetAxisXUnitText
  (params (Text :type Text))
  (Variables|/Script/Text3D.Text3DComponent|SetText (Variables|Default|GetAxisXUnit) Text))

(event Custom|SetAxisYUnitText
  (params (Text :type Text))
  (Variables|/Script/Text3D.Text3DComponent|SetText (Variables|Default|GetAxisYUnit) Text))

(event Custom|AddAxisXValue
  (params (AxisXValue :type String))
  (Utilities|Array|Add (Variables|Default|GetAxisXValues) AxisXValue))

(event Custom|AddAxisYValue
  (params (AxisYValue :type String))
  (Utilities|Array|Add (Variables|Default|GetAxisYValues) AxisYValue))

(fn ConstructionScript
  (CallFunction|Update))

(fn GetOriginLocation
  (return (Variables|Default|GetOriginLocation)))

(fn GetAxisXDirection
  (return (Transformation|GetActorForwardVector)))

(fn GetAxisXEndLocation
  (return (+ (CallFunction|GetOriginLocation) (* (CallFunction|GetAxisXDirection) (.x (Variables|Default|GetGridSize))))))

(fn GetAxisYDirection
  (return (* (Transformation|GetActorRightVector) -1.0)))

(fn GetAxisYEndLocation
  (return (+ (CallFunction|GetOriginLocation) (* (CallFunction|GetAxisYDirection) (.y (Variables|Default|GetGridSize))))))

(fn GetAxisEndLocation
  (return (+ (CallFunction|GetAxisXEndLocation) (* (CallFunction|GetAxisYDirection) (.y (Variables|Default|GetGridSize))))))