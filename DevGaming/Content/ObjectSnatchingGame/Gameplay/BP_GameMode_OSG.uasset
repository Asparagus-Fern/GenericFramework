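; Game mode for the object snatching game that tracks connected players and decides when a match can start.
; Each login restarts a short waiting timer, debouncing joins before checking for at least two players.
; A passing check calls ServerStartGame on BP_GameState_OSG; a failing one calls GameOver, which is still an empty stub.
; Logouts remove the player and rerun the check immediately, so remaining players can trigger the start call again.
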(event Custom|OnWaitingCompleted
  (CallFunction|CheckCanPlayGame)
  (Utilities|Time|ClearandInvalidateTimerbyHandle (Variables|Default|GetWaitingPlayerTimerHandle)))

(event Custom|ResetWaitingPlayerTimerHandle
  (Utilities|FlowControl|Sequence
    (:then_0
      (Utilities|Time|ClearandInvalidateTimerbyHandle (Variables|Default|GetWaitingPlayerTimerHandle)))
    (:then_1
      (bind _returnvalue (Utilities|Time|SetTimerbyEvent (delegate Custom|OnWaitingCompleted) 2.0))
      (Variables|Default|SetWaitingPlayerTimerHandle _returnvalue))))

(event Custom|GameOver)

(event Custom|GameStart
  (bind _returnvalue (Class|BPFunctionsGameplay|GetGameStatebyClass "/DevGaming/ObjectSnatchingGame/Gameplay/BP_GameState_OSG.BP_GameState_OSG_C"))
  (Utilities|IsValid _returnvalue
    (:Is%20Valid
      (Default|ServerStartGame _returnvalue))))

(event Custom|CheckCanPlayGame
  (if (CallFunction|CanPlayGame)
    (CallFunction|GameStart)
    (else
      (CallFunction|GameOver))))

(event EventPostLogin
  (params (NewPlayer :type Player%20Controller%20Object%20Reference))
  (Utilities|Array|Add (Variables|Default|GetPlayers) NewPlayer)
  (CallFunction|ResetWaitingPlayerTimerHandle))

(event EventOnLogout
  (params (ExitingController :type Controller%20Object%20Reference))
  (bind _asplayer_controller (Utilities|Casting|CastToPlayerController ExitingController))
  (Utilities|Array|RemoveItem (Variables|Default|GetPlayers) _asplayer_controller)
  (CallFunction|CheckCanPlayGame))

(fn ConstructionScript)

(fn CanPlayGame
  (return (>= (Utilities|Array|Length (Variables|Default|GetPlayers)) 2)))