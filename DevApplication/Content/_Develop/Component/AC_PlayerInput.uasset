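; Player input component that routes Enhanced Input actions to its owning actor.
; Move, turn and zoom values are forwarded as location, rotation and zoom messages on the owner, which handles the response.
; Jump start and completion cast the owner to Character to call Jump and StopJumping, so jumping only works on Character owners.
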(event Input|EnhancedActionEvents|EnhancedInputActionIA_Move
  (params (ActionValue :type Vector%202D%20Structure) (ElapsedSeconds :type Float%20%28double-precision%29) (TriggeredSeconds :type Float%20%28double-precision%29) (InputAction :type Input%20Action%20Object%20Reference :default "/DevCore/Input/MovementActions/IA_Move.IA_Move"))
  (Class|PawnInterface|AddLocation(Message) (Components|GetOwner) ActionValue))

(event Input|EnhancedActionEvents|EnhancedInputActionIA_Turn
  (params (ActionValue :type Vector%202D%20Structure) (ElapsedSeconds :type Float%20%28double-precision%29) (TriggeredSeconds :type Float%20%28double-precision%29) (InputAction :type Input%20Action%20Object%20Reference :default "/DevCore/Input/MovementActions/IA_Turn.IA_Turn"))
  (Class|PawnInterface|AddRotation(Message) (Components|GetOwner) ActionValue))

(event Input|EnhancedActionEvents|EnhancedInputActionIA_Zoom
  (params (ActionValue :type Float%20%28double-precision%29) (ElapsedSeconds :type Float%20%28double-precision%29) (TriggeredSeconds :type Float%20%28double-precision%29) (InputAction :type Input%20Action%20Object%20Reference :default "/DevCore/Input/MovementActions/IA_Zoom.IA_Zoom"))
  (Class|PawnInterface|AddZoom(Message) (Components|GetOwner) ActionValue))

(event Input|EnhancedActionEvents|EnhancedInputActionIA_Jump
  (params (ActionValue :type Float%20%28double-precision%29) (ElapsedSeconds :type Float%20%28double-precision%29) (TriggeredSeconds :type Float%20%28double-precision%29) (InputAction :type Input%20Action%20Object%20Reference :default "/DevCore/Input/MovementActions/IA_Jump.IA_Jump"))
  (bind _returnvalue (Components|GetOwner))
  (:Started
    (bind _ascharacter (Utilities|Casting|CastToCharacter _returnvalue))
    (Character|Jump _ascharacter))
  (:Completed
    (bind _ascharacter_2 (Utilities|Casting|CastToCharacter _returnvalue))
    (Character|StopJumping _ascharacter_2)))