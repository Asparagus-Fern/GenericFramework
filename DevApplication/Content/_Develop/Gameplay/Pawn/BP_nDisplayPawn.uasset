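; BP_nDisplayPawn is a player pawn, named for nDisplay, that moves, turns and zooms through Enhanced Input actions.
; The move, turn and zoom actions pass their values to AddLocation, AddRotation and AddZoom, which are defined outside this graph.
; BeginPlay caches directly attached actors, and each turn input then sets their rotation to the pawn's GetRotation result.
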(event Custom|UpdateAttachedChildren
  ;[1 0 0.6562] Comment
  (for _array_element (Variables|Default|GetAttachedChildren)
    (bind _returnvalue (Class|PawnInputMovementInterface|GetRotation))
    (Transformation|SetActorRotation _array_element _returnvalue)))

(event Input|EnhancedActionEvents|EnhancedInputActionIA_Move
  (params (ActionValue :type Vector%202D%20Structure) (ElapsedSeconds :type Float%20%28double-precision%29) (TriggeredSeconds :type Float%20%28double-precision%29) (InputAction :type Input%20Action%20Object%20Reference :default "/DevCore/Input/MovementActions/IA_Move.IA_Move"))
  (Class|PawnInputMovementInterface|AddLocation ActionValue))

(event Input|EnhancedActionEvents|EnhancedInputActionIA_Turn
  (params (ActionValue :type Vector%202D%20Structure) (ElapsedSeconds :type Float%20%28double-precision%29) (TriggeredSeconds :type Float%20%28double-precision%29) (InputAction :type Input%20Action%20Object%20Reference :default "/DevCore/Input/MovementActions/IA_Turn.IA_Turn"))
  (Class|PawnInputMovementInterface|AddRotation ActionValue)
  (CallFunction|UpdateAttachedChildren))

(event Input|EnhancedActionEvents|EnhancedInputActionIA_Zoom
  (params (ActionValue :type Float%20%28double-precision%29) (ElapsedSeconds :type Float%20%28double-precision%29) (TriggeredSeconds :type Float%20%28double-precision%29) (InputAction :type Input%20Action%20Object%20Reference :default "/DevCore/Input/MovementActions/IA_Zoom.IA_Zoom"))
  (Class|PawnInputMovementInterface|AddZoom ActionValue))

(event EventBeginPlay
  ;[1 0 0.6562] Comment
  (Variables|Default|SetAttachedChildren (Actor|GetAttachedActors true false)))

(fn ConstructionScript)