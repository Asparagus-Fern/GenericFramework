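; BP_HomeRoam is a pawn-folder Blueprint holding test logic for hosting and joining multiplayer sessions, none of which runs.
; Two unconnected chains find lobby sessions and join the first or second result.
; A third creates a session and opens L_Room as a listen server.
; Each chain prints its success or failure, and the construction script is empty.
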(event Input|KeyboardEvents|1
  (params (Key :type Key%20Structure :default "None")))

(event Input|KeyboardEvents|2
  (params (Key :type Key%20Structure :default "None")))

(event Input|KeyboardEvents|3
  (params (Key :type Key%20Structure :default "None")))

(fn ConstructionScript)