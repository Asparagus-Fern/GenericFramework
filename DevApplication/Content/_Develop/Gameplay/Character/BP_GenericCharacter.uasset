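; BP_GenericCharacter is a character Blueprint that routes Enhanced Input for moving, turning and zooming.
; Move and Turn input pass straight to AddLocation and AddRotation.
; Zoom applies only in the third-person rig from InputMovementComponent, scaling the X of a GameplayCamera Vector3 variable proportionally, 10% per input unit.
; An unconnected FlipFlop for switching between first- and third-person rigs never runs.
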(event Input|EnhancedActionEvents|EnhancedInputActionIA_Move
  (params (ActionValue :type Vector%202D%20Structure) (ElapsedSeconds :type Float%20%28double-precision%29) (TriggeredSeconds :type Float%20%28double-precision%29) (InputAction :type Input%20Action%20Object%20Reference :default "/DevCore/Input/MovementActions/IA_Move.IA_Move"))
  (Class|PawnInputMovementInterface|AddLocation ActionValue))

(event Input|EnhancedActionEvents|EnhancedInputActionIA_Turn
  (params (ActionValue :type Vector%202D%20Structure) (ElapsedSeconds :type Float%20%28double-precision%29) (TriggeredSeconds :type Float%20%28double-precision%29) (InputAction :type Input%20Action%20Object%20Reference :default "/DevCore/Input/MovementActions/IA_Turn.IA_Turn"))
  (Class|PawnInputMovementInterface|AddRotation ActionValue))

(event Input|EnhancedActionEvents|EnhancedInputActionIA_Zoom
  (params (ActionValue :type Float%20%28double-precision%29) (ElapsedSeconds :type Float%20%28double-precision%29) (TriggeredSeconds :type Float%20%28double-precision%29) (InputAction :type Input%20Action%20Object%20Reference :default "/DevCore/Input/MovementActions/IA_Zoom.IA_Zoom"))
  (Class|PawnInputMovementInterface|AddZoom ActionValue))

(event EventAddZoom
  (params (InValue :type Float%20%28single-precision%29))
  (bind _gameplaycamera (Variables|Default|GetGameplayCamera))
  (bind _returnvalue (Class|GameplayCameraComponent|GetInitialVariableTable _gameplaycamera))
  (switch Utilities|FlowControl|Switch|SwitchonECameraRig (Class|PawnInputMovementComponent|GetActiveCameraRig (Variables|Default|GetInputMovementComponent))
    (:ThirdPerson
      (bind _returnvalue_2 (Class|BlueprintCameraVariableTableFunctionLibrary|GetVector3CameraVariable _returnvalue "/CameraModule/CVC_ThirdPerson.CVC_ThirdPerson.Vector3dCameraVariable_0"))
      (Class|BlueprintCameraVariableTableFunctionLibrary|SetVector3CameraVariable _returnvalue "/CameraModule/CVC_ThirdPerson.CVC_ThirdPerson.Vector3dCameraVariable_0" (Math|Vector|MakeVector (+ (.x _returnvalue_2) (* (.x _returnvalue_2) 0.1 InValue)) 0.0 0.0)))))

(event Input|KeyboardEvents|1
  (params (Key :type Key%20Structure :default "None")))

(fn ConstructionScript)