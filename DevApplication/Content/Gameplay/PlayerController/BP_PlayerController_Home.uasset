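; Home-screen player controller that registers the main menu button collection on BeginPlay and unregisters it on EndPlay.
; Number-key debug hooks test online sessions, printing results to screen.
; They create a listen-server session from a settings view model and open Main_Server, or search sessions through both FindSessions and a view-model-based search.
; Older join and create session paths and a UI-only input mode call remain unconnected.
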(event EventBeginPlay
  (bind _returnvalue (Class|BPFunctionsGenericButtonWidget|RegisterButtonCollectionbyClass self "/DevApplication/Blueprint/ButtonCollection/BP_ButtonCollection_MainMenu.BP_ButtonCollection_MainMenu_C" true))
  (bind _output_get (Variables|Default|SetMainMenu _returnvalue)))

(event EventEndPlay
  (params (EndPlayReason :type EEndPlayReason%20Enum :default "Destroyed"))
  (Class|BPFunctionsGenericButtonWidget|UnRegisterButtonCollection (Variables|Default|GetMainMenu)))

(event Input|KeyboardEvents|4
  (params (Key :type Key%20Structure :default "None"))
  (:Pressed
    (Development|PrintString "4")
    (bind _searchsettingviewmodel (|FindSessionsbyClass (Class|BPFunctionNetwork|ToUniqueNetworkID(PlayerController) self) "/DevApplication/UMG/Session/VM_SessionSearchSettings_Search.VM_SessionSearchSettings_Search_C")
      (:OnSuccess
        (Development|PrintString "success")
        (Class|SessionSearchSettingViewModel|RefreshSessionSearchResults _searchsettingviewmodel)
        (Development|PrintString (Utilities|String|ToString(Integer) (Utilities|Array|Length (Class|SessionSearchSettingViewModel|GetSessionSearchResults _searchsettingviewmodel)))))
      (:OnFail
        (Development|PrintString "Fail")))))

(event Input|KeyboardEvents|1
  (params (Key :type Key%20Structure :default "None"))
  (:Pressed
    (Development|PrintString "1")
    (|SessionbyClass (Class|BPFunctionNetwork|ToUniqueNetworkID(PlayerController) self) "Test" "/DevApplication/UMG/Session/VM_SessionSettings_ListenServer.VM_SessionSettings_ListenServer_C" true
      (:OnSuccess
        (Development|PrintString "success")
        (Game|OpenLevel(byObjectReference) "/DevApplication/Map/Main_Server.Main_Server" true "listen"))
      (:OnFail
        (Development|PrintString "Fail")))))

(event Input|KeyboardEvents|2
  (params (Key :type Key%20Structure :default "None")))

(event Input|KeyboardEvents|3
  (params (Key :type Key%20Structure :default "None"))
  (:Pressed
    (Development|PrintString "3")
    (bind _results (|FindSessions self 10 false false)
      (:OnSuccess
        (if (Utilities|Array|IsValidIndex _results)
          (Development|PrintString (Utilities|String|Append "Current Player :" (Utilities|String|ToString(Integer) (Class|FindSessionsCallbackProxy|GetCurrentPlayers (Utilities|Array|Get(acopy) _results))) " 
Max Player :" (Utilities|String|ToString(Integer) (Class|FindSessionsCallbackProxy|GetMaxPlayers (Utilities|Array|Get(acopy) _results))) " 
Server Name : " (Class|FindSessionsCallbackProxy|GetServerName (Utilities|Array|Get(acopy) _results))) true true "(R=0.000000,G=0.660000,B=1.000000,A=1.000000)" 2e+01)
          (else
            (Development|PrintString "InValid Index"))))
      (:OnFailure
        (Development|PrintString "Fail")))))

(fn ConstructionScript)