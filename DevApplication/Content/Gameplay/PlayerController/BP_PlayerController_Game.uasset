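; BP_PlayerController_Game is the gameplay player controller that sets game-only input and handles the escape menu toggle.
; BeginPlay switches the input mode to game only.
; When the escape menu input action completes, it lazily registers BP_ButtonCollection_EscMenu as an active button collection and caches it in EscMenu.
; Later presses flip that cached collection's active state instead of registering a new one.
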(event Input|EnhancedActionEvents|EnhancedInputActionIA_TiggerEscMenu
  (params (ActionValue :type Boolean) (ElapsedSeconds :type Float%20%28double-precision%29) (TriggeredSeconds :type Float%20%28double-precision%29) (InputAction :type Input%20Action%20Object%20Reference :default "/DevCore/Input/ShortcutActions/IA_TiggerEscMenu.IA_TiggerEscMenu"))
  (:Completed
    (bind _escmenu (Variables|Default|GetEscMenu)
      (:then
        (Class|GenericButtonCollection|SetIsActived (Variables|Default|GetEscMenu) (not (Class|GenericButtonCollection|GetIsActived _escmenu))))
      (:else
        (bind _returnvalue (Class|BPFunctionsGenericButtonWidget|RegisterButtonCollectionbyClass self "/DevApplication/Blueprint/ButtonCollection/BP_ButtonCollection_EscMenu.BP_ButtonCollection_EscMenu_C" true))
        (Variables|Default|SetEscMenu _returnvalue)))))

(event EventBeginPlay
  (Input|SetInputModeGameOnly self false))

(event EventEndPlay
  (params (EndPlayReason :type EEndPlayReason%20Enum :default "Destroyed")))

(fn ConstructionScript)