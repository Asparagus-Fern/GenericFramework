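; Button collection for the game menu, handling selection of the Start, Join Session, Settings, About and Exit buttons.
; Start sets up a session, opens Main_Server as a listen server and unregisters this collection; About is an empty stub.
; Join Session and Settings register child button collections while selected, and Exit opens a confirmation popup that quits on Yes.
; Child collection unregistration or popup cancel deselects the MainMenu button group.
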(event Custom|OnSelectionChanged_UI.Button.GameMenu.Settings
  (params (Selection :type Boolean))
  (if Selection
    (bind _returnvalue (Class|BPFunctionsGenericButtonWidget|RegisterButtonCollectionbyClass (Class|GenericButtonCollection|GetOwnerPlayer) "/DevApplication/Blueprint/ButtonCollection/BP_ButtonCollection_Settings.BP_ButtonCollection_Settings_C" true))
    (EventDispatchers|AssignOnButtonCollectionUnRegister _returnvalue (delegate Custom|OnSettingButtonCollectionUnRegister_Event))
    (elif (.ReturnValue (Class|BPFunctionsGenericButtonWidget|IsButtonCollectionRegistered _returnvalue))
      (if (.IsRegistered (Class|BPFunctionsGenericButtonWidget|IsButtonCollectionRegistered _returnvalue))
        (Class|BPFunctionsGenericButtonWidget|UnRegisterButtonCollection _returnvalue)))))

(event Custom|OnSelectionChanged_UI.Button.GameMenu.About
  (params (Selection :type Boolean)))

(event Custom|OnSelectionChanged_UI.Button.GameMenu.Exit
  (params (Selection :type Boolean))
  (if Selection
    (bind _returnvalue (UserInterface|CreateWidget "/DevApplication/UMG/Popup/Dialog/WBP_PopupDialog_ExitGame.WBP_PopupDialog_ExitGame_C" (Class|GenericButtonCollection|GetOwnerPlayer)))
    (EventDispatchers|AssignBPDelegateonPopupResultSubmitted _returnvalue (delegate Custom|OnExitGameResultSubmitted_Event))
    (|AsyncOpenGenericWidget _returnvalue)
    (else
      (Utilities|IsValid _returnvalue
        (:Is%20Valid
          (EventDispatchers|UnbindallEventsfromBPDelegateonPopupResultSubmitted _returnvalue)
          (|AsyncCloseGenericWidget _returnvalue))))))

(event Custom|OnJoinSessionButtonCollectionUnRegister_Event
  (bind _returnvalue (Class|GenericButtonCollection|GetButtonGroup "(TagName=\"UI.Button.MainMenu\")"))
  (Utilities|IsValid _returnvalue
    (:Is%20Valid
      (Class|GenericButtonGroup|DeselectAll _returnvalue))))

(event Custom|OnExitGameResultSubmitted_Event
  (params (InPopupResult :type Gameplay%20Tag%20Structure))
  (bind _returnvalue (Class|GenericButtonCollection|GetButtonGroup "(TagName=\"UI.Button.MainMenu\")"))
  (|SwitchGameplayTag InPopupResult
    (:Result.Generic.Yes
      (Development|ExecuteConsoleCommand "exit" (Class|GenericButtonCollection|GetOwnerPlayer)))
    (:Result.Generic.Cancel
      (Utilities|IsValid _returnvalue
        (:Is%20Valid
          (Class|GenericButtonGroup|DeselectAll _returnvalue))))))

(event Custom|OnSettingButtonCollectionUnRegister_Event
  (bind _returnvalue (Class|GenericButtonCollection|GetButtonGroup "(TagName=\"UI.Button.MainMenu\")"))
  (Utilities|IsValid _returnvalue
    (:Is%20Valid
      (Class|GenericButtonGroup|DeselectAll _returnvalue))))

(event Custom|OnSelectionChanged_UI.Button.GameMenu.Start
  (params (Selection :type Boolean))
  (if Selection
    (Utilities|FlowControl|Sequence
      (:then_0
        (|Session (Class|BPFunctionNetwork|ToUniqueNetworkID(PlayerController) (Class|GenericButtonCollection|GetOwnerPlayer)) (Variables|Default|GetSessionSettings)
          (:OnSuccess
            (Game|OpenLevel(byObjectReference) "/DevApplication/Map/Main_Server.Main_Server" true "listen"))))
      (:then_1
        (Class|BPFunctionsGenericButtonWidget|UnRegisterButtonCollection self)))))

(event Custom|OnSelectionChanged_UI.Button.GameMenu.JoinSession
  (params (Selection :type Boolean))
  (if Selection
    (bind _returnvalue (Class|BPFunctionsGenericButtonWidget|RegisterButtonCollectionbyClass (Class|GenericButtonCollection|GetOwnerPlayer) "/DevApplication/Blueprint/ButtonCollection/BP_ButtonCollection_JoinSession.BP_ButtonCollection_JoinSession_C" true))
    (EventDispatchers|AssignOnButtonCollectionUnRegister _returnvalue (delegate Custom|OnJoinSessionButtonCollectionUnRegister_Event))
    (elif (.ReturnValue (Class|BPFunctionsGenericButtonWidget|IsButtonCollectionRegistered _returnvalue))
      (if (.IsRegistered (Class|BPFunctionsGenericButtonWidget|IsButtonCollectionRegistered _returnvalue))
        (Class|BPFunctionsGenericButtonWidget|UnRegisterButtonCollection _returnvalue)))))