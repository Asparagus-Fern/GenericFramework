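; Escape-menu button collection that pauses the game and shows the cursor while active, restoring game-only input when inactive.
; Per-tag selection handlers deactivate the menu for Continue, register a Settings sub-collection, or open async confirmation popups for Exit to Home and Exit Game; About is empty.
; Popup results switch on gameplay tags to load the home level or quit; cancelling, or unregistering Settings, deselects the button group.
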(event EventHandleonActived
  (bind _returnvalue (Class|GenericButtonCollection|GetOwnerPlayer))
  (Variables|/Script/Engine.PlayerController|SetbShowMouseCursor _returnvalue true)
  (Input|SetInputModeGameandUI _returnvalue 0 "DoNotLock" true false)
  (Game|SetGamePaused true))

(event EventHandleonInactived
  (bind _returnvalue (Class|GenericButtonCollection|GetOwnerPlayer))
  (Variables|/Script/Engine.PlayerController|SetbShowMouseCursor _returnvalue false)
  (Input|SetInputModeGameOnly _returnvalue false)
  (Game|SetGamePaused false))

(event Custom|OnSelectionChanged_UI.Button.EscMenu.Continue
  (params (Selection :type Boolean))
  (if Selection
    (Class|GenericButtonCollection|SetIsActived false)))

(event Custom|OnSelectionChanged_UI.Button.EscMenu.Settings
  (params (Selection :type Boolean))
  (if Selection
    (bind _returnvalue (Class|BPFunctionsGenericButtonWidget|RegisterButtonCollectionbyClass (Class|GenericButtonCollection|GetOwnerPlayer) "/DevApplication/Blueprint/ButtonCollection/BP_ButtonCollection_Settings.BP_ButtonCollection_Settings_C" true))
    (EventDispatchers|AssignOnButtonCollectionUnRegister _returnvalue (delegate Custom|OnSettingButtonCollectionUnRegister_Event))
    (elif (.ReturnValue (Class|BPFunctionsGenericButtonWidget|IsButtonCollectionRegistered _returnvalue))
      (if (.IsRegistered (Class|BPFunctionsGenericButtonWidget|IsButtonCollectionRegistered _returnvalue))
        (Class|BPFunctionsGenericButtonWidget|UnRegisterButtonCollection _returnvalue)))))

(event Custom|OnSelectionChanged_UI.Button.EscMenu.About
  (params (Selection :type Boolean)))

(event Custom|OnSelectionChanged_UI.Button.EscMenu.ExitToHome
  (params (Selection :type Boolean))
  (if Selection
    (bind _returnvalue (UserInterface|CreateWidget "/DevApplication/UMG/Popup/Dialog/WBP_PopupDialog_ExitToHome.WBP_PopupDialog_ExitToHome_C" (Class|GenericButtonCollection|GetOwnerPlayer)))
    (EventDispatchers|AssignBPDelegateonPopupResultSubmitted _returnvalue (delegate Custom|OnExitToHomeResultSubmitted_Event))
    (|AsyncOpenGenericWidget _returnvalue)
    (else
      (Utilities|IsValid _returnvalue
        (:Is%20Valid
          (EventDispatchers|UnbindallEventsfromBPDelegateonPopupResultSubmitted _returnvalue)
          (|AsyncCloseGenericWidget _returnvalue))))))

(event Custom|OnSelectionChanged_UI.Button.EscMenu.ExitGame
  (params (Selection :type Boolean))
  (if Selection
    (bind _returnvalue (UserInterface|CreateWidget "/DevApplication/UMG/Popup/Dialog/WBP_PopupDialog_ExitGame.WBP_PopupDialog_ExitGame_C" (Class|GenericButtonCollection|GetOwnerPlayer)))
    (EventDispatchers|AssignBPDelegateonPopupResultSubmitted _returnvalue (delegate Custom|OnExitGameResultSubmitted_Event))
    (|AsyncOpenGenericWidget _returnvalue)
    (else
      (Utilities|IsValid _returnvalue
        (:Is%20Valid
          (EventDispatchers|UnbindallEventsfromBPDelegateonPopupResultSubmitted _returnvalue)
          (|AsyncCloseGenericWidget _returnvalue))))))

(event Custom|OnExitGameResultSubmitted_Event
  (params (InPopupResult :type Gameplay%20Tag%20Structure))
  (bind _returnvalue (Class|GenericButtonCollection|GetButtonGroup "(TagName=\"UI.Button.EscMenu\")"))
  (|SwitchGameplayTag InPopupResult
    (:Result.Generic.Yes
      (Development|ExecuteConsoleCommand "exit" (Class|GenericButtonCollection|GetOwnerPlayer)))
    (:Result.Generic.Cancel
      (Utilities|IsValid _returnvalue
        (:Is%20Valid
          (Class|GenericButtonGroup|DeselectAll _returnvalue))))))

(event Custom|OnExitToHomeResultSubmitted_Event
  (params (InPopupResult :type Gameplay%20Tag%20Structure))
  (bind _returnvalue (Class|GenericButtonCollection|GetButtonGroup "(TagName=\"UI.Button.EscMenu\")"))
  (|SwitchGameplayTag InPopupResult
    (:Result.Generic.Yes
      (Game|OpenLevel(byObjectReference) "/DevApplication/Map/Main_Home.Main_Home")
      (Class|BPFunctionsGenericButtonWidget|UnRegisterButtonCollection self))
    (:Result.Generic.Cancel
      (Utilities|IsValid _returnvalue
        (:Is%20Valid
          (Class|GenericButtonGroup|DeselectAll _returnvalue))))))

(event Custom|OnSettingButtonCollectionUnRegister_Event
  (bind _returnvalue (Class|GenericButtonCollection|GetButtonGroup "(TagName=\"UI.Button.EscMenu\")"))
  (Utilities|IsValid _returnvalue
    (:Is%20Valid
      (Class|GenericButtonGroup|DeselectAll _returnvalue))))