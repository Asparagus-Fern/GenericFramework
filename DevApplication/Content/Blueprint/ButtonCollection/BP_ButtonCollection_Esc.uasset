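; Button collection for the Esc pause menu, with entries for continue, settings tabs, about, and exit.
; Activation shows the cursor, switches to game-and-UI input and pauses the game; deactivation reverses this.
; Selection events are named after UI gameplay tags: Continue deactivates the menu and Settings Return deselects all in the Esc button group.
; The other selection handlers are empty stubs.
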(event EventHandleonActived
  (bind _returnvalue (Game|GetPlayerController 0))
  (Variables|/Script/Engine.PlayerController|SetbShowMouseCursor _returnvalue true)
  (Input|SetInputModeGameandUI _returnvalue 0 "DoNotLock" true false)
  (Game|SetGamePaused true))

(event EventHandleonInactived
  (bind _returnvalue (Game|GetPlayerController 0))
  (Variables|/Script/Engine.PlayerController|SetbShowMouseCursor _returnvalue false)
  (Input|SetInputModeGameOnly _returnvalue false)
  (Game|SetGamePaused false))

(event Custom|OnSelectionChanged_UI.Button.MenuEsc.Settings.Return
  (params (Selection :type Boolean))
  (bind _returnvalue (Class|GenericButtonCollection|GetButtonGroup "(TagName=\"UI.Button.Esc\")"))
  (Utilities|IsValid _returnvalue
    (:Is%20Valid
      (Class|GenericButtonGroup|DeselectAll _returnvalue))))

(event Custom|OnSelectionChanged_UI.Button.MenuEsc.Continue
  (params (Selection :type Boolean))
  (Class|GenericButtonCollection|SetIsActived false))

(event Custom|OnSelectionChanged_UI.Button.MenuEsc.Settings
  (params (Selection :type Boolean)))

(event Custom|OnSelectionChanged_UI.Button.MenuEsc.AboutUs
  (params (Selection :type Boolean)))

(event Custom|OnSelectionChanged_UI.Button.MenuEsc.ExitToHome
  (params (Selection :type Boolean)))

(event Custom|OnSelectionChanged_UI.Button.MenuEsc.ExitGame
  (params (Selection :type Boolean)))

(event Custom|OnSelectionChanged_UI.Button.MenuEsc.Settings.Game
  (params (Selection :type Boolean)))

(event Custom|OnSelectionChanged_UI.Button.MenuEsc.Settings.Video
  (params (Selection :type Boolean)))

(event Custom|OnSelectionChanged_UI.Button.MenuEsc.Settings.Sound
  (params (Selection :type Boolean)))

(event Custom|OnSelectionChanged_UI.Button.MenuEsc.Settings.Keyboard
  (params (Selection :type Boolean)))

(event Custom|OnSelectionChanged_UI.Button.MenuEsc.Settings.Controller
  (params (Selection :type Boolean)))