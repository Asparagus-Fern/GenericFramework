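; AC_GraphComponent is an actor component that holds a segment layout for a row and column graph, apparently an unfinished prototype.
; Its UpdateRow event is empty, and the only logic is disconnected, so it never runs.
; That unused logic steps through each segment's count and draws red debug boxes from the owner's location plus StartLocation, spacing them along +X for rows or -Y for columns.
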(event Custom|UpdateRow)