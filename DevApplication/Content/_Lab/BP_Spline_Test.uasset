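; Experimental spline actor that tiles random instanced meshes along its path, rebuilt from the Construction Script.
; SpawnInstances creates one instanced component per entry in Meshes, with scale factors fitting each mesh to MainMesh bounds.
; It steps along the spline one unit at a time, closing segments when length or height change exceeds scaled bounds.
; Each segment gets a yaw-only instance at its midpoint, producing steps on slopes.
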(event Custom|SpawnInstances
  (bind _meshes (Variables|Default|GetMeshes))
  (bind _output (Utilities|Array|Get(acopy) _meshes))
  (for _array_element (Actor|GetComponentsByClass "/Script/Engine.InstancedStaticMeshComponent")
    (Components|DestroyComponent _array_element))
  (Utilities|Array|Clear (Variables|Default|GetInstanceStaticMeshComponents))
  (for _array_element_2 (Variables|Default|GetMeshes)
    (bind _returnvalue (AddComponent|AddInstancedStaticMeshComponent false))
    (Components|StaticMesh|SetStaticMesh _returnvalue _array_element_2)
    (Utilities|Array|Add (Variables|Default|GetInstanceStaticMeshComponents) _returnvalue))
  (Utilities|IsValid _output
    (:Is%20Valid
      (Variables|Default|GetMainMesh
        (:then
          _)
        (:else
          (Variables|Default|SetMainMesh _output)))
      (Utilities|Array|Clear (Variables|Default|GetBoundingBoxScales))
      (for _array_element_3 (Variables|Default|GetMeshes)
        (Utilities|Array|Add (Variables|Default|GetBoundingBoxScales) (/ (CallFunction|GetMainMeshBoundingBox) (- (.max (StaticMesh|GetBoundingBox _array_element_3)) (.min (StaticMesh|GetBoundingBox _array_element_3))))))
      (if (< (Variables|Default|GetNextDistance) (Spline|GetSplineLength (Variables|Default|GetSpline))) :!label _label
        (if (CallFunction|CanCreateInstance)
          (CallFunction|AddRandomInstance (CallFunction|GetInstanceLocation) (CallFunction|GetInstanceRotation) (CallFunction|GetInstanceScale))
          (Variables|Default|SetCurrentDistance (Variables|Default|GetNextDistance))
          (goto _label)
          (else
            (Math|Float|IncrementFloat (Variables|Default|GetNextDistance)
              (:%20%20
                (goto _label)))))))))

(fn ConstructionScript
  (CallFunction|SpawnInstances))

(fn DebugPoint
  (params (Distance :type Float%20%28single-precision%29))
  (Rendering|Debug|DrawDebugPoint :Position (Spline|GetLocationatDistanceAlongSpline (Variables|Default|GetSpline) Distance "World") :Size 5e+01 :Duration 1e+01))

(fn GetMainMeshBoundingBox
  (bind _mainmesh (Variables|Default|GetMainMesh))
  (bind _returnvalue (StaticMesh|GetBoundingBox _mainmesh))
  (return (- (.max _returnvalue) (.min _returnvalue))))

(fn CanCreateInstance
  (if (> (Math|Float|Absolute(Float) (- (.z (Spline|GetLocationatDistanceAlongSpline (Variables|Default|GetSpline) (Variables|Default|GetNextDistance) "World")) (.z (Spline|GetLocationatDistanceAlongSpline (Variables|Default|GetSpline) (Variables|Default|GetCurrentDistance) "World")))) (* (* (.z (CallFunction|GetMainMeshBoundingBox)) (.z (Variables|Default|GetScale))) (LocalVariables|GetAlpha)))
    (return true)
    (else
      (return (> (- (Variables|Default|GetNextDistance) (Variables|Default|GetCurrentDistance)) (* (.x (CallFunction|GetMainMeshBoundingBox)) (.x (Variables|Default|GetScale))))))))

(fn GetInstanceLocation
  (return (Spline|GetLocationatDistanceAlongSpline (Variables|Default|GetSpline) (+ (/ (- (Variables|Default|GetNextDistance) (Variables|Default|GetCurrentDistance)) 2.0) (Variables|Default|GetCurrentDistance)) "World")))

(fn GetInstanceRotation
  (return (Math|Rotator|MakeRotator 0.0 0.0 (.yaw (Math|Rotator|FindLookatRotation (Spline|GetLocationatDistanceAlongSpline (Variables|Default|GetSpline) (Variables|Default|GetNextDistance) "World") (Spline|GetLocationatDistanceAlongSpline (Variables|Default|GetSpline) (Variables|Default|GetCurrentDistance) "World"))))))

(fn GetInstanceScale
  (return (Variables|Default|GetScale)))

(fn AddRandomInstance
  (params (Location :type Vector) (Rotation :type Rotator) (Scale :type Vector))
  (bind _instancestaticmeshcomponents (Variables|Default|GetInstanceStaticMeshComponents))
  (bind (_outitem _outindex) (Utilities|Array|Random _instancestaticmeshcomponents))
  (Components|InstancedStaticMesh|AddInstance _outitem (Math|Transform|MakeTransform Location Rotation (* Scale (Utilities|Array|Get(acopy) (Variables|Default|GetBoundingBoxScales) _outindex))) true))