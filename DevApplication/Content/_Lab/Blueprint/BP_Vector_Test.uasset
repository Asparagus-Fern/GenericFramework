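; BP_Vector_Test is a lab Blueprint that visualizes vector math with splines built in its construction script.
; One spline runs from A to B in local space.
; A second runs from A to the A-to-B direction, yawed by Angle and scaled to half the distance over cos(Angle).
; That isosceles-apex vector is not offset by A, so it is measured from the local origin.
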(event EventBeginPlay)

(event Collision|EventActorBeginOverlap
  (params (OtherActor :type Actor%20Object%20Reference)))

(event EventTick
  (params (DeltaSeconds :type Float%20%28single-precision%29)))

(fn ConstructionScript
  (bind _a (Variables|Default|GetA))
  (bind _b (Variables|Default|GetB))
  (bind _angle (Variables|Default|GetAngle))
  (Utilities|FlowControl|Sequence
    (:then_0
      (bind _returnvalue (AddComponent|AddSplineComponent false))
      (Spline|ClearSplinePoints _returnvalue true)
      (Spline|AddSplinePoint _returnvalue (Variables|Default|GetA) "Local" true)
      (Spline|AddSplinePoint _returnvalue (Variables|Default|GetB) "Local" true))
    (:then_1
      (bind _returnvalue_2 (AddComponent|AddSplineComponent false))
      (Spline|ClearSplinePoints _returnvalue_2 true)
      (Spline|AddSplinePoint _returnvalue_2 (Variables|Default|GetA) "Local" true)
      (Spline|AddSplinePoint _returnvalue_2 (* (Math|Vector|RotateVector (Math|Vector|Normalize (- _b _a)) (Math|Rotator|MakeRotator 0.0 0.0 _angle)) (/ (/ (Math|Vector|Distance(Vector) _b _a) 2.0) (Math|Trig|Cos(Degrees) _angle))) "Local" true))))