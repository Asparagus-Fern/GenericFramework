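; BP_SimpleNiagaraSpline is a lab Blueprint pairing a Niagara component with a spline, intended to move the effect along the path.
; An unconnected DOFloat tween samples the spline by time in local space to set the effect's relative location, looping over Duration until IsStop is set.
; A separate unconnected FlipFlop toggles Niagara activation.
; BeginPlay and the construction script are empty, so none of this logic runs.
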(event EventBeginPlay)

(event Input|KeyboardEvents|2
  (params (Key :type Key%20Structure)))

(fn ConstructionScript)